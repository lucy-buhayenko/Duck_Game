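; BP_egg is an egg pickup that plays a sound and destroys itself when BP_paperHERO overlaps its sphere.
; The sphere's begin-overlap event casts to the hero, so other actors are ignored.
; It also carries character input logic: BeginPlay adds the IA_paperMap mapping context when a PlayerController possesses it, and IA_jump calls Jump on both Started and Triggered.
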(event `self.ReceiveBeginPlay`
  (bind _asplayer_controller (cast `PlayerController` (`self.GetController`)))
  (`EnhancedInputSubsystemInterface.AddMappingContext` (pcsubsystem `EnhancedInputLocalPlayerSubsystem` _asplayer_controller) "/Game/input/IA_paperMap.IA_paperMap" 0 (struct)))

(event `EnhancedInput|/Game/input/IA_jump`
  (params (ActionValue :type Boolean) (ElapsedSeconds :type "Float (double-precision)") (TriggeredSeconds :type "Float (double-precision)") (InputAction :type "InputAction Object Reference" :default "/Game/input/IA_jump.IA_jump"))
  (:`Started`
    (`self.Jump`)))

(event `EnhancedInput|/Game/input/IA_jump`
  (params (ActionValue :type Boolean) (ElapsedSeconds :type "Float (double-precision)") (TriggeredSeconds :type "Float (double-precision)") (InputAction :type "InputAction Object Reference" :default "/Game/input/IA_jump.IA_jump"))
  (:`Triggered`
    (`self.Jump`)))

(event `self.Sphere.OnComponentBeginOverlap`
  (params (OverlappedComponent :type "PrimitiveComponent Object Reference") (OtherActor :type "Actor Object Reference") (OtherComp :type "PrimitiveComponent Object Reference") (OtherBodyIndex :type Integer) (bFromSweep :type Boolean) (SweepResult :type "HitResult Structure (by ref)"))
  (cast `/Game/Character/BP_paperHERO` OtherActor)
  (`GameplayStatics.PlaySound2D` "/Game/HUD/egg.egg" 1.0 1.0 0.0 null null)
  (`self.K2_DestroyActor`))

(fn `UserConstructionScript`)