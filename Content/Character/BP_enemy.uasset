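; BP_enemy is a Paper2D enemy character that constantly moves forward on Tick and jumps whenever its Box1 trigger overlaps something.
; When its Box overlaps BP_paperHERO, it waits briefly, shows the Lose widget, then, once only, plays a losing sound and opens Game3 after a delay.
; It also has Enhanced Input jump bindings that require a PlayerController, while its flipbook-switching logic is unconnected and never runs.
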(event `self.ReceiveBeginPlay`
  (bind _asplayer_controller (cast `PlayerController` (`self.GetController`)))
  (`EnhancedInputSubsystemInterface.AddMappingContext` (pcsubsystem `EnhancedInputLocalPlayerSubsystem` _asplayer_controller) "/Game/input/IA_paperMap.IA_paperMap" 0 (struct)))

(event `EnhancedInput|/Game/input/IA_jump`
  (params (ActionValue :type Boolean) (ElapsedSeconds :type "Float (double-precision)") (TriggeredSeconds :type "Float (double-precision)") (InputAction :type "InputAction Object Reference" :default "/Game/input/IA_jump.IA_jump"))
  (:`Started`
    (`self.Jump`)))

(event `EnhancedInput|/Game/input/IA_jump`
  (params (ActionValue :type Boolean) (ElapsedSeconds :type "Float (double-precision)") (TriggeredSeconds :type "Float (double-precision)") (InputAction :type "InputAction Object Reference" :default "/Game/input/IA_jump.IA_jump"))
  (:`Triggered`
    (`self.Jump`)))

(event `self.ReceiveTick`
  (params (DeltaSeconds :type "Float (single-precision)"))
  (`self.AddMovementInput` (`self.GetActorForwardVector`) 0.75))

(event `self.Box.OnComponentBeginOverlap`
  (params (OverlappedComponent :type "PrimitiveComponent Object Reference") (OtherActor :type "Actor Object Reference") (OtherComp :type "PrimitiveComponent Object Reference") (OtherBodyIndex :type Integer) (bFromSweep :type Boolean) (SweepResult :type "HitResult Structure (by ref)"))
  (cast `/Game/Character/BP_paperHERO` OtherActor)
  (`KismetSystemLibrary.Delay` 0.3)
  (bind _returnvalue (`|CreateWidget` "/Game/Character/lose.lose_C"))
  (`UserWidget.AddToViewport` _returnvalue 0)
  (`/Engine/EditorBlueprintResources/StandardMacros.DoOnce` false
    (:`Completed`
      (`GameplayStatics.PlaySound2D` "/Game/HUD/loseBanjo.loseBanjo" 1.0 1.0 0.0 null null)
      (`KismetSystemLibrary.Delay` 1.5)
      (`GameplayStatics.OpenLevelBySoftObjectPtr` "/Game/mask/game3.game3"))))

(event `self.Box1.OnComponentBeginOverlap`
  (params (OverlappedComponent :type "PrimitiveComponent Object Reference") (OtherActor :type "Actor Object Reference") (OtherComp :type "PrimitiveComponent Object Reference") (OtherBodyIndex :type Integer) (bFromSweep :type Boolean) (SweepResult :type "HitResult Structure (by ref)"))
  (`self.Jump`))

(fn `UserConstructionScript`)