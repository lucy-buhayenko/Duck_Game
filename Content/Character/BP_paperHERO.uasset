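; BP_paperHERO is a Paper2D player character for a side-scrolling game, with Enhanced Input move and jump.
; Movement runs along world X, and control rotation yaw flips to face the travel direction.
; Tick picks the run, idle or jump flipbook from ground state and velocity, keeping the current one while falling.
; Tick also pins the spring arm to a fixed world height, so the camera ignores jumps.
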(event `self.ReceiveBeginPlay`
  (bind _asplayer_controller (cast `PlayerController` (`self.GetController`)))
  (`EnhancedInputSubsystemInterface.AddMappingContext` (pcsubsystem `EnhancedInputLocalPlayerSubsystem` _asplayer_controller) "/Game/input/IA_paperMap.IA_paperMap" 0 (struct)))

(event `EnhancedInput|/Game/input/IA_jump`
  (params (ActionValue :type Boolean) (ElapsedSeconds :type "Float (double-precision)") (TriggeredSeconds :type "Float (double-precision)") (InputAction :type "InputAction Object Reference" :default "/Game/input/IA_jump.IA_jump"))
  (:`Started`
    (`self.Jump`)))

(event `EnhancedInput|/Game/input/IA_move`
  (params (ActionValue :type "Float (double-precision)") (ElapsedSeconds :type "Float (double-precision)") (TriggeredSeconds :type "Float (double-precision)") (InputAction :type "InputAction Object Reference" :default "/Game/input/IA_move.IA_move"))
  (:`Triggered`
    (`self.AddMovementInput` (1.0 0.0 0.0) ActionValue)
    (`Controller.SetControlRotation` (`self.GetController`) (select `bool` (> ActionValue 0.0) :`false` (`KismetMathLibrary.MakeRotator` 0.0 0.0 180.0) :`true` (`KismetMathLibrary.MakeRotator` 0.0)))))

(event `self.ReceiveTick`
  (params (DeltaSeconds :type "Float (single-precision)"))
  (bind (_returnvalue_x _returnvalue_y _returnvalue_z) (`KismetMathLibrary.BreakVector` (`self.GetVelocity`)))
  (bind (_returnvalue_x_2 _returnvalue_y_2) (`KismetMathLibrary.BreakVector` (`self.K2_GetActorLocation`)))
  (`|ExecutionSequence`
    (:`then_0`
      (if (`NavMovementComponent.IsMovingOnGround` (`self.CharacterMovement`))
        (if (> (`KismetMathLibrary.VSize` (`self.GetVelocity`)) 0.0)
          (`PaperFlipbookComponent.SetFlipbook` (`self.Sprite`) "/Game/runBetter.runBetter")
          (else
            (`PaperFlipbookComponent.SetFlipbook` (`self.Sprite`) "/Game/idlebreathe.idlebreathe")))
        (elif (not (< _returnvalue_z 0.0))
          (`PaperFlipbookComponent.SetFlipbook` (`self.Sprite`) "/Game/jumpDuck.jumpDuck"))))
    (:`then_1`
      (`SceneComponent.K2_SetWorldLocation` (`self.SpringArm`) (`KismetMathLibrary.MakeVector` _returnvalue_x_2 _returnvalue_y_2 -1900.0) false false))))

(fn `UserConstructionScript`)